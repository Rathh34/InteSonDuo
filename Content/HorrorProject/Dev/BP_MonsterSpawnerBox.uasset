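; BP_MonsterSpawnerBox is a one-shot trigger box that stages a monster reveal and starts a chase when the player overlaps it.
; It unhides a referenced monster, disables input and uses a timeline to swing the camera to a fixed rotation.
; Afterwards it restores input and shows a "Run" prompt.
; After a short delay it starts the monster's AI tree and switches ambience audio to Chase.
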(event OnComponentBeginOverlap(Box)
  (params (OverlappedComponent :type Primitive%20Component%20Object%20Reference) (OtherActor :type Actor%20Object%20Reference) (OtherComp :type Primitive%20Component%20Object%20Reference) (OtherBodyIndex :type Integer) (bFromSweep :type Boolean) (SweepResult :type Hit%20Result%20Structure%20%28by%20ref%29))
  (bind _asbp_third_person_character (Utilities|Casting|CastToBP_ThirdPersonCharacter OtherActor))
  (Utilities|FlowControl|DoOnce false
    (:Completed
      (bind _monstertomakevisible (Variables|Default|GetMonsterToMakeVisible)
        (:then
          (Rendering|SetActorHiddenInGame _monstertomakevisible false))
        (:else
          _))
      (Variables|Default|SetAs%20ThirdPersonCharacter _asbp_third_person_character)
      (Input|DisableInput _asbp_third_person_character 0)
      (Variables|Default|SetRotationRef (Pawn|GetControlRotation (Game|GetPlayerController 0) :!class /Script/Engine.Controller))
      (bind _alpha (Timeline|Timeline PlayFromStart)
        (:Update
          (Pawn|SetControlRotation (Game|GetPlayerController 0) (Math|Rotator|Lerp(Rotator) (Math|Rotator|MakeRotator 0.0 0.0 (.yaw (Variables|Default|GetRotationRef))) "0.000000,-90.000000,0.000000" _alpha true)))
        (:Finished
          (Input|EnableInput (Variables|Default|GetAs%20ThirdPersonCharacter) 0)
          (Rendering|Components|TextRender|SetText (Variables|/Game/HorrorProject/Dev/Tuto/WBP_Tuto.WBP_Tuto_C|GetTXT_Tuto (Variables|/Game/HorrorProject/UI/HUD_Player.HUD_Player_C|GetWBP_Tuto (Variables|/Game/ThirdPerson/Blueprints/BP_ThirdPersonCharacter.BP_ThirdPersonCharacter_C|GetHUDref (Variables|Default|GetAs%20ThirdPersonCharacter)))) "Run")
          (UserInterface|Animation|PlayAnimation (Variables|/Game/HorrorProject/UI/HUD_Player.HUD_Player_C|GetWBP_Tuto (Variables|/Game/ThirdPerson/Blueprints/BP_ThirdPersonCharacter.BP_ThirdPersonCharacter_C|GetHUDref (Variables|Default|GetAs%20ThirdPersonCharacter))) (Variables|/Game/HorrorProject/Dev/Tuto/WBP_Tuto.WBP_Tuto_C|GetAppear (Variables|/Game/HorrorProject/UI/HUD_Player.HUD_Player_C|GetWBP_Tuto (Variables|/Game/ThirdPerson/Blueprints/BP_ThirdPersonCharacter.BP_ThirdPersonCharacter_C|GetHUDref (Variables|Default|GetAs%20ThirdPersonCharacter)))) 0.0 1 "Forward" 1.0 false)
          (Utilities|FlowControl|Delay 1.5)
          (bind _asaic_monster (Utilities|Casting|CastToAIC_Monster (Pawn|GetController (Variables|Default|GetMonsterToMakeVisible))))
          (Default|StartTree _asaic_monster)
          (Class|GameAudioDirectorComponent|SetAmbienceState (Variables|/Game/ThirdPerson/Blueprints/BP_ThirdPersonCharacter.BP_ThirdPersonCharacter_C|GetGameAudioDirector (Variables|Default|GetAs%20ThirdPersonCharacter)) "Chase" 1.0))))))

(fn ConstructionScript)