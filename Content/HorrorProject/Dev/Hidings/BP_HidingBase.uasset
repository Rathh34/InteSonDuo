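; BP_HidingBase is a base hiding place that lets the player hide at its HidingSpot.
; Box overlaps with BP_Player toggle CanInteract, which gates the Interaction event.
; Interaction on a player not already hidden makes Cube block Pawns, stores the target and current location on the player, then calls Hide with itself and its hide/unhide animations.
; QuitHiding is an empty event here.
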(event OnComponentBeginOverlap(Box)
  (params (OverlappedComponent :type Primitive%20Component%20Object%20Reference) (OtherActor :type Actor%20Object%20Reference) (OtherComp :type Primitive%20Component%20Object%20Reference) (OtherBodyIndex :type Integer) (bFromSweep :type Boolean) (SweepResult :type Hit%20Result%20Structure%20%28by%20ref%29))
  (Utilities|Casting|CastToBP_Player OtherActor)
  (Variables|Default|SetCanInteract true))

(event OnComponentEndOverlap(Box)
  (params (OverlappedComponent :type Primitive%20Component%20Object%20Reference) (OtherActor :type Actor%20Object%20Reference) (OtherComp :type Primitive%20Component%20Object%20Reference) (OtherBodyIndex :type Integer))
  (Utilities|Casting|CastToBP_Player OtherActor)
  (Variables|Default|SetCanInteract false))

(event Custom|QuitHiding)

(event EventInteraction
  (params (Player :type BP%20Player%20Object%20Reference))
  (bind _returnvalue (Transformation|GetActorLocation Player))
  (if (Variables|Default|GetCanInteract)
    (if (not (Variables|/Game/HorrorProject/Core/Characters/BP_Player.BP_Player_C|GetbIsHidden Player))
      (Collision|SetCollisionResponsetoChannel (Variables|Default|GetCube) "ECC_Pawn" "ECR_Block")
      (Variables|/Game/HorrorProject/Core/Characters/BP_Player.BP_Player_C|SetTargetLocation Player (Transformation|GetWorldLocation (Variables|Default|GetHidingSpot)))
      (Variables|/Game/HorrorProject/Core/Characters/BP_Player.BP_Player_C|SetZLoc Player (.Z (Math|Vector|BreakVector _returnvalue)))
      (Variables|/Game/HorrorProject/Core/Characters/BP_Player.BP_Player_C|SetCurrentLoc Player _returnvalue)
      (Default|Hide Player (Variables|Default|GetUnhide%20Anim) (Variables|Default|GetHide%20Anim) self))))

(fn ConstructionScript)