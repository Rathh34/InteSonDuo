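; BP_Locker is a locker hiding spot whose door animates as the player enters and leaves.
; It extends a parent hiding class, calling the parent logic first on Interact and QuitHiding.
; When interaction is allowed and the player is not hidden, a timeline rotates the static mesh open by interpolating its relative rotation.
; Quitting hiding reverses that timeline from the end to swing the mesh back.
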(event EventInteract
  (params (Player :type BP%20Third%20Person%20Character%20Object%20Reference))
  (|CallParentFunction Player)
  (if (Variables|Default|GetCanInteract)
    (if (not (Variables|/Game/ThirdPerson/Blueprints/BP_ThirdPersonCharacter.BP_ThirdPersonCharacter_C|GetbIsHidden Player))
      (bind _alpha (Timeline|Timeline PlayFromStart)
        (:Update
          (Transformation|SetRelativeRotation (Variables|Default|GetStaticMesh) (Math|Rotator|Lerp(Rotator) "0, 0, 0" "0.000000,-100.000000,0.000000" _alpha) false false))))))

(event Collision|EventActorBeginOverlap
  (params (OtherActor :type Actor%20Object%20Reference))
  (|CallParentFunction OtherActor) ; This node is disabled and will not be called.\nDrag off pins to build functionality.
)

(event EventTick
  (params (DeltaSeconds :type Float%20%28single-precision%29))
  (|CallParentFunction DeltaSeconds) ; This node is disabled and will not be called.\nDrag off pins to build functionality.
)

(event EventQuitHiding
  (|CallParentFunction)
  (bind _alpha (Timeline|Timeline ReverseFromEnd)
    (:Update
      (Transformation|SetRelativeRotation (Variables|Default|GetStaticMesh) (Math|Rotator|Lerp(Rotator) "0, 0, 0" "0.000000,-100.000000,0.000000" _alpha) false false))))

(fn ConstructionScript
  (|CallParentFunction))