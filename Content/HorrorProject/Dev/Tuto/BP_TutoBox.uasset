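; BP_TutoBox is a tutorial trigger that shows a text prompt on the player's HUD the first time its Box component is overlapped.
; It sets TextToDisplay on the WBPTuto widget, reached through the player character's HUD reference, and plays its Appear animation.
; If a ToDelete actor is valid, it destroys that actor after a short delay.
; The overlapping actor is not checked.
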(event OnComponentBeginOverlap(Box)
  (params (OverlappedComponent :type Primitive%20Component%20Object%20Reference) (OtherActor :type Actor%20Object%20Reference) (OtherComp :type Primitive%20Component%20Object%20Reference) (OtherBodyIndex :type Integer) (bFromSweep :type Boolean) (SweepResult :type Hit%20Result%20Structure%20%28by%20ref%29))
  (bind _returnvalue (Game|Player|GetPlayerPawn 0))
  (bind _asbp_third_person_character (Utilities|Casting|CastToBP_ThirdPersonCharacter _returnvalue))
  (bind _hudref (Variables|/Game/ThirdPerson/Blueprints/BP_ThirdPersonCharacter.BP_ThirdPersonCharacter_C|GetHUDref _asbp_third_person_character))
  (bind _wbp_tuto (Variables|/Game/HorrorProject/UI/HUD_Player.HUD_Player_C|GetWBP_Tuto _hudref))
  (Utilities|FlowControl|DoOnce false
    (:Completed
      (Variables|/Script/UMG.TextBlock|SetText (Variables|/Game/HorrorProject/Dev/Tuto/WBP_Tuto.WBP_Tuto_C|GetTXT_Tuto _wbp_tuto) (Variables|Default|GetTextToDisplay))
      (UserInterface|Animation|PlayAnimation _wbp_tuto (Variables|/Game/HorrorProject/Dev/Tuto/WBP_Tuto.WBP_Tuto_C|GetAppear _wbp_tuto) 0.0 1 "Forward" 1.0 false)
      (bind _todelete (Variables|Default|GetToDelete)
        (:then
          (Utilities|FlowControl|Delay 1.0)
          (Actor|DestroyActor _todelete))
        (:else)))))

(fn ConstructionScript)